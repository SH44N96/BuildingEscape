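; Openable door actor that swings around its yaw axis in response to events from OpenDoor.
; The DoorSwing timeline drives an angle that is combined with the rotation cached at BeginPlay, so the swing is relative to the door's placement.
; OnClose plays the timeline forward and OnOpen reverses it.
; An event track on the timeline plays the Door_Lock sound at the door's location.
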(event OnClose(OpenDoor)
  (bind _open_angle (Timeline|Door%20Swing Play)
    (:Update
      (Transformation|SetActorRotation (Math|Rotator|CombineRotators (Math|Rotator|MakeRotator 0.0 0.0 _open_angle) (Variables|Default|GetInitial%20Rotation))))
    (:Sound%20Timing
      (Audio|PlaySoundatLocation "/Game/Audio/Door_Lock.Door_Lock" (Transformation|GetActorLocation) "0, 0, 0" 1.0 1.0 0.0 0 0 0))))

(event OnOpen(OpenDoor)
  (bind _open_angle (Timeline|Door%20Swing Reverse)
    (:Update
      (Transformation|SetActorRotation (Math|Rotator|CombineRotators (Math|Rotator|MakeRotator 0.0 0.0 _open_angle) (Variables|Default|GetInitial%20Rotation))))
    (:Sound%20Timing
      (Audio|PlaySoundatLocation "/Game/Audio/Door_Lock.Door_Lock" (Transformation|GetActorLocation) "0, 0, 0" 1.0 1.0 0.0 0 0 0))))

(event EventBeginPlay
  (Variables|Default|SetInitial%20Rotation (Transformation|GetActorRotation)))

(fn ConstructionScript)